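; GM_Game is a game mode that manages the player HUD and the game over screen.
; On BeginPlay it creates the PlayerHUD widget, stores it as CurrentHUD and adds it to the viewport.
; Its GameOver event disables player input, swaps the HUD for a GameOver widget, switches to UI-only input and shows the mouse cursor.
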(event `self.ReceiveBeginPlay`
  (bind _returnvalue (`|CreateWidget` "/Game/Widgets/PlayerHUD.PlayerHUD_C"))
  (bind _output_get (set `self.CurrentHUD` _returnvalue))
  (`UserWidget.AddToViewport` _output_get 0))

(event `GameOver`
  (bind _returnvalue (`GameplayStatics.GetPlayerController` 0))
  (`self.DisableInput` (`GameplayStatics.GetPlayerCharacter` 0) (`GameplayStatics.GetPlayerController` 0))
  (`Widget.RemoveFromParent` (`self.CurrentHUD`))
  (bind _returnvalue_2 (`|CreateWidget` "/Game/Widgets/GameOver.GameOver_C"))
  (`UserWidget.AddToViewport` _returnvalue_2 0)
  (`WidgetBlueprintLibrary.SetInputMode_UIOnlyEx` _returnvalue _returnvalue_2)
  (set `PlayerController.bShowMouseCursor` true _returnvalue))

(fn `UserConstructionScript`)