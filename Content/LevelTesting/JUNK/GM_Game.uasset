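; Game mode, by its name, that handles the HUD at start and the switch to a game-over screen.
; BeginPlay creates a widget, but sets CurrentHUD to None rather than to that widget before adding it to the viewport.
; The GameOver event disables player 0's input, removes CurrentHUD, shows a second widget, and switches to UI-only input with a visible cursor.
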(event `self.ReceiveBeginPlay`
  (bind _returnvalue (`|CreateWidget` null))
  (bind (_output_get _output_get_2) (set `self.CurrentHUD` null _returnvalue))
  (`UserWidget.AddToViewport` _output_get_2 0))

(event `GameOver`
  (bind _returnvalue (`GameplayStatics.GetPlayerController` 0))
  (`self.DisableInput` (`GameplayStatics.GetPlayerCharacter` 0) (`GameplayStatics.GetPlayerController` 0))
  (`Widget.RemoveFromParent` (`.CurrentHUD` (`self.CurrentHUD`)))
  (bind _returnvalue_2 (`|CreateWidget` null))
  (`UserWidget.AddToViewport` _returnvalue_2 0)
  (`WidgetBlueprintLibrary.SetInputMode_UIOnlyEx` _returnvalue _returnvalue_2)
  (set `PlayerController.bShowMouseCursor` true _returnvalue))

(fn `UserConstructionScript`)