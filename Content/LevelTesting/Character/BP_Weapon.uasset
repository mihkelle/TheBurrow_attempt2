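; BP_Weapon is a weapon actor that the player's TestCharacter can pick up and equip.
; PickUp swaps weapons: any currently equipped one is detached and moved to this weapon's root location and rotation.
; It then stores itself as the character's EquipWeapon and snaps to the R_HoldItem socket on the character mesh.
; The event always acts on player 0, and nothing in this Blueprint calls it.
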(event `/Game/LevelTesting/Character/WeaponPickup.PickUp`
  (bind _defaultsceneroot (`self.DefaultSceneRoot`))
  (bind _astest_character (cast `/Game/LevelTesting/Character/TestCharacter` (`GameplayStatics.GetPlayerCharacter` 0) :!pure true))
  (bind _equipweapon (`/Game/LevelTesting/Character/TestCharacter.EquipWeapon` (cast `/Game/LevelTesting/Character/TestCharacter` (`GameplayStatics.GetPlayerCharacter` 0) :!pure true)))
  (`/Engine/EditorBlueprintResources/StandardMacros.IsValid` _equipweapon
    (:`Is Valid`
      ;[1 1 1] Weapon Switch
      (`self.K2_DetachFromActor` _equipweapon "KeepRelative" "KeepRelative" "KeepRelative")
      (`self.K2_SetActorLocationAndRotation` _equipweapon (`SceneComponent.K2_GetComponentLocation` _defaultsceneroot) (`SceneComponent.K2_GetComponentRotation` _defaultsceneroot) false false))
    (:`Is Not Valid`
      _))
  (set `/Game/LevelTesting/Character/TestCharacter.EquipWeapon` self _astest_character)
  (`self.K2_AttachToComponent` (`Character.Mesh` _astest_character) "R_HoldItem" "SnapToTarget" "SnapToTarget" "KeepRelative"))

(fn `UserConstructionScript`)