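; BP_DoorExit is an exit door that brings up the UMG_Exit menu for the player.
; Overlapping Door_Collison enables input on the door for the player character, and leaving disables it.
; Pressing Interact shows the widget with a mouse cursor, pauses the game and turns off the hero's HUD.
; An OpenDoor event duplicates that sequence for other Blueprints to call, while CalculateHealth is an empty stub.
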(event `self.Door_Collison.OnComponentBeginOverlap`
  (params (OverlappedComponent :type "PrimitiveComponent Object Reference") (OtherActor :type "Actor Object Reference") (OtherComp :type "PrimitiveComponent Object Reference") (OtherBodyIndex :type Integer) (bFromSweep :type Boolean) (SweepResult :type "HitResult Structure (by ref)"))
  ;[1 1 1] En-/disable Inputs
  (if (== OtherActor (`GameplayStatics.GetPlayerCharacter` 0))
    (`self.EnableInput` (`GameplayStatics.GetPlayerController` 0))))

(event `self.Door_Collison.OnComponentEndOverlap`
  (params (OverlappedComponent :type "PrimitiveComponent Object Reference") (OtherActor :type "Actor Object Reference") (OtherComp :type "PrimitiveComponent Object Reference") (OtherBodyIndex :type Integer))
  ;[1 1 1] En-/disable Inputs
  (if (== OtherActor (`GameplayStatics.GetPlayerCharacter` 0))
    (`self.DisableInput` (`GameplayStatics.GetPlayerController` 0))))

(event `InputAction|Interact`
  (params (Key :type "Key Structure"))
  (bind _returnvalue (`GameplayStatics.GetPlayerController` 0))
  ;[1 1 1] Interact toob esile menüü, mis võimaldab exit
  (:`Pressed`
    (bind _returnvalue_2 (`|CreateWidget` "/Game/MyAssets/UMG/Widgets/UMG_Exit.UMG_Exit_C"))
    (`UserWidget.AddToViewport` _returnvalue_2 0)
    (`WidgetBlueprintLibrary.SetInputMode_GameAndUIEx` _returnvalue null)
    (set `PlayerController.bShowMouseCursor` true _returnvalue)
    (`GameplayStatics.SetGamePaused` true)
    (`/Game/MyAssets/Blueprints/BP_HeroCharacter.ToggleHUDoff` (cast `/Game/MyAssets/Blueprints/BP_HeroCharacter` (`GameplayStatics.GetPlayerCharacter` 0) :!pure true))))

(event `OpenDoor`
  (bind _returnvalue (`GameplayStatics.GetPlayerController` 0))
  ;[1 1 1] Custom Event for opening door from other BP-s
  (bind _returnvalue_2 (`|CreateWidget` "/Game/MyAssets/UMG/Widgets/UMG_Exit.UMG_Exit_C"))
  (`UserWidget.AddToViewport` _returnvalue_2 0)
  (`WidgetBlueprintLibrary.SetInputMode_GameAndUIEx` _returnvalue null)
  (set `PlayerController.bShowMouseCursor` true _returnvalue)
  (`GameplayStatics.SetGamePaused` true)
  (`/Game/MyAssets/Blueprints/BP_HeroCharacter.ToggleHUDoff` (cast `/Game/MyAssets/Blueprints/BP_HeroCharacter` (`GameplayStatics.GetPlayerCharacter` 0) :!pure true)))

(fn `CalculateHealth`
  (params (delta :type "Float (double-precision)")))

(fn `UserConstructionScript`)