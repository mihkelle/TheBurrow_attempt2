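; BP_Potion is a pickup actor that lets the player collect a potion.
; A Box overlap enables input on the actor while the player stands inside and disables it on exit.
; Pressing Interact then destroys the potion, calls AdjustPotionNumber on BP_HeroCharacter and sets its PickupSlot3 flag.
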(event `self.Box.OnComponentBeginOverlap`
  (params (OverlappedComponent :type "PrimitiveComponent Object Reference") (OtherActor :type "Actor Object Reference") (OtherComp :type "PrimitiveComponent Object Reference") (OtherBodyIndex :type Integer) (bFromSweep :type Boolean) (SweepResult :type "HitResult Structure (by ref)"))
  ;[1 1 1] Enable input on collision
  (if (== OtherActor (`GameplayStatics.GetPlayerCharacter` 0))
    (`self.EnableInput` (`GameplayStatics.GetPlayerController` 0))))

(event `self.Box.OnComponentEndOverlap`
  (params (OverlappedComponent :type "PrimitiveComponent Object Reference") (OtherActor :type "Actor Object Reference") (OtherComp :type "PrimitiveComponent Object Reference") (OtherBodyIndex :type Integer))
  ;[1 1 1] Enable input on collision
  (if (== OtherActor (`GameplayStatics.GetPlayerCharacter` 0))
    (`self.DisableInput` (`GameplayStatics.GetPlayerController` 0))))

(event `InputAction|Interact`
  (params (Key :type "Key Structure"))
  ;[1 1 1] Pickup item
  (:`Pressed`
    (bind _asbp_hero_character (cast `/Game/MyAssets/Blueprints/BP_HeroCharacter` (`GameplayStatics.GetPlayerCharacter` 0)))
    (`self.K2_DestroyActor`)
    (`/Game/MyAssets/Blueprints/BP_HeroCharacter.AdjustPotionNumber` _asbp_hero_character)
    (set `/Game/MyAssets/Blueprints/BP_HeroCharacter.PickupSlot3` true _asbp_hero_character)))

(fn `UserConstructionScript`)