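; BP_Door is a breakable door that takes health changes and drops a potion when destroyed.
; AffectHealth passes a delta to CalculateHealth, plays a hit sound, and at zero health destroys the door, plays a destruction sound and spawns BP_Potion at its location.
; Both sounds play at world origin.
; The collision overlap toggles player input on the door, though no input events are bound here.
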(event `self.Door_Collison.OnComponentBeginOverlap`
  (params (OverlappedComponent :type "PrimitiveComponent Object Reference") (OtherActor :type "Actor Object Reference") (OtherComp :type "PrimitiveComponent Object Reference") (OtherBodyIndex :type Integer) (bFromSweep :type Boolean) (SweepResult :type "HitResult Structure (by ref)"))
  ;[1 1 1] En-/disable Inputs
  (if (== OtherActor (`GameplayStatics.GetPlayerCharacter` 0))
    (`self.EnableInput` (`GameplayStatics.GetPlayerController` 0))))

(event `self.Door_Collison.OnComponentEndOverlap`
  (params (OverlappedComponent :type "PrimitiveComponent Object Reference") (OtherActor :type "Actor Object Reference") (OtherComp :type "PrimitiveComponent Object Reference") (OtherBodyIndex :type Integer))
  ;[1 1 1] En-/disable Inputs
  (if (== OtherActor (`GameplayStatics.GetPlayerCharacter` 0))
    (`self.DisableInput` (`GameplayStatics.GetPlayerController` 0))))

(event `/Game/MyAssets/Blueprints/I_Damagable.AffectHealth`
  (params (Delta :type "Float (single-precision)"))
  ;[1 1 1] Receive damage and die
  (`self.CalculateHealth` Delta)
  (`GameplayStatics.PlaySoundAtLocation` "/Game/LevelTesting/Audio/AudioFiles/SFX_DoorBreak_Cue.SFX_DoorBreak_Cue" (0.0 0.0 0.0) (struct) 1.0 1.0 0.0 null null null)
  (`KismetSystemLibrary.PrintString` "HITT!")
  (if (`self.isDead`)
    (`self.K2_DestroyActor`)
    (`GameplayStatics.PlaySoundAtLocation` "/Game/LevelTesting/Audio/AudioFiles/BB_SFX_DestroyDoor.BB_SFX_DestroyDoor" (0.0 0.0 0.0) (struct) 1.0 1.0 0.0 null null null)
    ;[1 1 1] Spawn loot pickup at death location
    (`|SpawnActorFromClass` "/Game/MyAssets/Blueprints/ItemBPs/BP_Potion.BP_Potion_C" (`KismetMathLibrary.MakeTransform` (`SceneComponent.K2_GetComponentLocation` (`self.Door`))) "Undefined" "OverrideRootScale" null null)))

(fn `CalculateHealth`
  (params (delta :type "Float (double-precision)"))
  (bind _output_get (set `self.Health` (+ (`self.Health`) delta)))
  (if (<= _output_get 0.0)
    (set `self.isDead` true)))

(fn `UserConstructionScript`)