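; Bone spear item that works as both a damaging object and a quest pickup for the player.
; On actor overlap it sends its Damage through BPI_Damagable to actors not tagged Friendly.
; A box trigger enables Interact input while the player is inside; a PickupSpear event offers the same pickup for line traces.
; Pickup sets the hero's slot 1 flag, plays a sound, destroys the spear and calls AdjustQuest0.
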(event `self.ReceiveActorBeginOverlap`
  (params (OtherActor :type "Actor Object Reference"))
  ;[1 1 1] Kontroll, kas löödav ese kasutab I_Damagable interface. Kui jah, siis saab teha dämmi, kui ei, siis ei
  (if (`KismetSystemLibrary.DoesImplementInterface` OtherActor "/Game/MyAssets/Blueprints/BPI_Damagable.BPI_Damagable_C")
    ;[1 1 1] Kas objektil on tag "Friendly"? Kui ei, siis tee dämmi. Kui jah, siis ei tee dämmi.
    (if (not (`self.ActorHasTag` OtherActor "Friendly"))
      (message `/Game/MyAssets/Blueprints/BPI_Damagable.AffectHealth` OtherActor (`self.Damage`)))))

(event `self.Box.OnComponentBeginOverlap`
  (params (OverlappedComponent :type "PrimitiveComponent Object Reference") (OtherActor :type "Actor Object Reference") (OtherComp :type "PrimitiveComponent Object Reference") (OtherBodyIndex :type Integer) (bFromSweep :type Boolean) (SweepResult :type "HitResult Structure (by ref)"))
  ;[1 1 1] Enable input on collision
  (if (== OtherActor (`GameplayStatics.GetPlayerCharacter` 0))
    (`self.EnableInput` (`GameplayStatics.GetPlayerController` 0))))

(event `self.Box.OnComponentEndOverlap`
  (params (OverlappedComponent :type "PrimitiveComponent Object Reference") (OtherActor :type "Actor Object Reference") (OtherComp :type "PrimitiveComponent Object Reference") (OtherBodyIndex :type Integer))
  ;[1 1 1] Enable input on collision
  (if (== OtherActor (`GameplayStatics.GetPlayerCharacter` 0))
    (`self.DisableInput` (`GameplayStatics.GetPlayerController` 0))))

(event `InputAction|Interact`
  (params (Key :type "Key Structure"))
  ;[1 1 1] Pickup item and update quest
  (:`Pressed`
    (bind _asbp_hero_character (cast `/Game/MyAssets/Blueprints/BP_HeroCharacter` (`GameplayStatics.GetPlayerCharacter` 0)))
    (set `/Game/MyAssets/Blueprints/BP_HeroCharacter.PIckupSlot1` true _asbp_hero_character)
    (`GameplayStatics.PlaySoundAtLocation` "/Game/Audio/Audio/AudioFiles/UI_Pickup1_Cue.UI_Pickup1_Cue" (`self.K2_GetActorLocation`) (struct) 1.0 1.0 0.0 null null null)
    (`self.K2_DestroyActor`)
    (`/Game/MyAssets/Blueprints/BP_HeroCharacter.AdjustQuest0` _asbp_hero_character)))

(event `PickupSpear`
  ;[1 1 1] Custom event for picking up spear by linetrace
  (bind _asbp_hero_character (cast `/Game/MyAssets/Blueprints/BP_HeroCharacter` (`GameplayStatics.GetPlayerCharacter` 0)))
  (set `/Game/MyAssets/Blueprints/BP_HeroCharacter.PIckupSlot1` true _asbp_hero_character)
  (`GameplayStatics.PlaySoundAtLocation` "/Game/Audio/Audio/AudioFiles/UI_Pickup1_Cue.UI_Pickup1_Cue" (`self.K2_GetActorLocation`) (struct) 1.0 1.0 0.0 null null null)
  (`self.K2_DestroyActor`)
  (`/Game/MyAssets/Blueprints/BP_HeroCharacter.AdjustQuest0` _asbp_hero_character))

(fn `UserConstructionScript`)