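; BP_FrogSkin is a pickup item for frog skins that advances a quest on the hero character.
; Its box overlap enables input for the player, so pressing Interact collects it.
; A separate PickupFrogSkin event, meant for line-trace pickup, repeats the same logic.
; Collection sets the hero's PickupSlot4 flag, plays a pickup sound, destroys the actor and calls AdjustQuest1.
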(event `self.Box.OnComponentBeginOverlap`
  (params (OverlappedComponent :type "PrimitiveComponent Object Reference") (OtherActor :type "Actor Object Reference") (OtherComp :type "PrimitiveComponent Object Reference") (OtherBodyIndex :type Integer) (bFromSweep :type Boolean) (SweepResult :type "HitResult Structure (by ref)"))
  ;[1 1 1] Enable input on collision
  (if (== OtherActor (`GameplayStatics.GetPlayerCharacter` 0))
    (`self.EnableInput` (`GameplayStatics.GetPlayerController` 0))))

(event `self.Box.OnComponentEndOverlap`
  (params (OverlappedComponent :type "PrimitiveComponent Object Reference") (OtherActor :type "Actor Object Reference") (OtherComp :type "PrimitiveComponent Object Reference") (OtherBodyIndex :type Integer))
  (if (== OtherActor (`GameplayStatics.GetPlayerCharacter` 0))
    (`self.DisableInput` (`GameplayStatics.GetPlayerController` 0))))

(event `InputAction|Interact`
  (params (Key :type "Key Structure"))
  ;[1 1 1] Pickup item and update quest
  (:`Pressed`
    (bind _asbp_hero_character (cast `/Game/MyAssets/Blueprints/BP_HeroCharacter` (`GameplayStatics.GetPlayerCharacter` 0)))
    (set `/Game/MyAssets/Blueprints/BP_HeroCharacter.PickupSlot4` true _asbp_hero_character)
    (`GameplayStatics.PlaySoundAtLocation` "/Game/Audio/Audio/AudioFiles/UI_Pickup1_Cue.UI_Pickup1_Cue" (`self.K2_GetActorLocation`) (struct) 1.0 1.0 0.0 null null null)
    (`self.K2_DestroyActor`)
    (`/Game/MyAssets/Blueprints/BP_HeroCharacter.AdjustQuest1` _asbp_hero_character)))

(event `PickupFrogSkin`
  ;[1 1 1] Custom Event for picking up frog skins by linetrace
  (bind _asbp_hero_character (cast `/Game/MyAssets/Blueprints/BP_HeroCharacter` (`GameplayStatics.GetPlayerCharacter` 0)))
  (set `/Game/MyAssets/Blueprints/BP_HeroCharacter.PickupSlot4` true _asbp_hero_character)
  (`GameplayStatics.PlaySoundAtLocation` "/Game/Audio/Audio/AudioFiles/UI_Pickup1_Cue.UI_Pickup1_Cue" (`self.K2_GetActorLocation`) (struct) 1.0 1.0 0.0 null null null)
  (`self.K2_DestroyActor`)
  (`/Game/MyAssets/Blueprints/BP_HeroCharacter.AdjustQuest1` _asbp_hero_character))

(fn `UserConstructionScript`)