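; AI enemy frog character that chases the hero, takes paw hits and drops frog skin on death.
; Perception updates Behavior Tree keys through its AI controller, toggles danger music, and uses a timer to forget lost targets.
; Damage counts only while a hero paw flag is active, clearing both flags; death updates kills, detaches the controller and destroys the actor.
; Construction tints the body; hero overlap only sets a flag, and hand-weapon spawning is disconnected.
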(event `self.AIPerception.OnTargetPerceptionUpdated`
  (params (Actor :type "Actor Object Reference") (Stimulus :type "AIStimulus Structure"))
  ;[1 1 1 1 14] Määratleb, millist mängijat nähti
  (set `self.PerceivedActor` Actor)
  (if (`.bSuccessfullySensed` (break `AIStimulus` Stimulus))
    ;[1 1 1 1 14] Nullib taimeri, kui mängija ilmub vaatevälja, ning BT võib jätkata tegevusi
    (`KismetSystemLibrary.K2_ClearAndInvalidateTimerHandle` (`self.TargetLostTimer`))
    ;[1 1 1] BT saab info, millist mängijat on nähtud
    (`/Game/MyAssets/Blueprints/AIC_ThirdPersonChar.UpdateTargetActorKey` (cast `/Game/MyAssets/Blueprints/AIC_ThirdPersonChar` (`self.GetController`) :!pure true) (`self.PerceivedActor`))
    ;[1 1 1] BT saab info, et mängija on nägemisraadiuses
    (`/Game/MyAssets/Blueprints/AIC_ThirdPersonChar.UpdateHasLineOfSightKey` (cast `/Game/MyAssets/Blueprints/AIC_ThirdPersonChar` (`self.GetController`) :!pure true) true)
    (`GameplayStatics.PlaySound2D` "/Game/LevelTesting/Audio/AudioFiles/Music/Stinger_Attack_Cue.Stinger_Attack_Cue" 1.0 1.0 0.0 "/Game/LevelTesting/Audio/Stinger_Conc.Stinger_Conc" null)
    (`GameplayStatics.SetSoundMixClassOverride` "/Game/LevelTesting/Audio/SM_Explore.SM_Explore" "/Game/LevelTesting/Audio/SC_MUSIC_GAME_DANGER.SC_MUSIC_GAME_DANGER" 1.0 1.0 1.5)
    (else
      ;[1 1 1] Kui AI ei näe mängijat 5 sek, siis kaotab huvi ja ei aja enam taga
      (bind _returnvalue (`KismetSystemLibrary.K2_SetTimerDelegate` (delegate `TargetLost`) 5.0))
      (set `self.TargetLostTimer` _returnvalue)
      ;[1 1 1 1 14] Anname BT-le info, et me ei näe enam mängijat, keda jälgisime
      (`/Game/MyAssets/Blueprints/AIC_ThirdPersonChar.UpdateHasLineOfSightKey` (cast `/Game/MyAssets/Blueprints/AIC_ThirdPersonChar` (`self.GetController`) :!pure true) false)
      (`GameplayStatics.ClearSoundMixClassOverride` "/Game/LevelTesting/Audio/SM_Explore.SM_Explore" "/Game/LevelTesting/Audio/SC_MUSIC_GAME_DANGER.SC_MUSIC_GAME_DANGER" 3.0))))

(event `TargetLost`
  ;[1 1 1] Kui AI ei näe mängijat 5 sek, siis kaotab huvi ja ei aja enam taga
  ;;[1 1 1 1 14] Kuna me ei anna uut väärtust, siis muutuja nullitakse
  (set `self.PerceivedActor` null)
  ;[1 1 1 1 14] Anname BT-le info, et nähtud mängija on unustatud
  ;;[1 1 1 1 14] Siin saame Target Actor = null
  (`/Game/MyAssets/Blueprints/AIC_ThirdPersonChar.UpdateTargetActorKey` (cast `/Game/MyAssets/Blueprints/AIC_ThirdPersonChar` (`self.GetController`) :!pure true) null))

(event `self.Capsule.OnComponentBeginOverlap`
  (params (OverlappedComponent :type "PrimitiveComponent Object Reference") (OtherActor :type "Actor Object Reference") (OtherComp :type "PrimitiveComponent Object Reference") (OtherBodyIndex :type Integer) (bFromSweep :type Boolean) (SweepResult :type "HitResult Structure (by ref)"))
  ;[1 1 1] Should trigger attack animation
  (cast `/Game/MyAssets/Blueprints/BP_HeroCharacter` OtherActor)
  (`KismetSystemLibrary.PrintString` "Overläp töötab!")
  (if (not (`self.HitHero`))
    (set `self.HitHero` true)
    (`KismetSystemLibrary.PrintString` "HitHeroActive" true true (struct :`R` 0.152456 :`G` 1.0 :`B` 0.086832 :`A` 1.0))))

(event `self.Capsule.OnComponentEndOverlap`
  (params (OverlappedComponent :type "PrimitiveComponent Object Reference") (OtherActor :type "Actor Object Reference") (OtherComp :type "PrimitiveComponent Object Reference") (OtherBodyIndex :type Integer))
  ;[1 1 1] Should trigger attack animation
  (cast `/Game/MyAssets/Blueprints/BP_HeroCharacter` OtherActor)
  (set `self.HitHero` false)
  (`KismetSystemLibrary.PrintString` "Hithero deactivated"))

(event `self.ReceiveAnyDamage`
  (params (Damage :type "Float (single-precision)") (DamageType :type "DamageType Object Reference") (InstigatedBy :type "Controller Object Reference") (DamageCauser :type "Actor Object Reference"))
  (bind _capsulecomponent (`self.CapsuleComponent`))
  ;[1 1 1] Hit by the hero
  (bind _asbp_hero_character (cast `/Game/MyAssets/Blueprints/BP_HeroCharacter` (`GameplayStatics.GetPlayerCharacter` 0)))
  (if (or (`/Game/MyAssets/Blueprints/BP_HeroCharacter.RightPawCanDamage` _asbp_hero_character) (`/Game/MyAssets/Blueprints/BP_HeroCharacter.LeftPawCanDamage` _asbp_hero_character))
    (set `/Game/MyAssets/Blueprints/BP_HeroCharacter.RightPawCanDamage` false _asbp_hero_character)
    (set `/Game/MyAssets/Blueprints/BP_HeroCharacter.LeftPawCanDamage` false _asbp_hero_character)
    ;[1 1 1] Receive damage and die
    (`self.CalculateHealth` Damage)
    (`KismetSystemLibrary.PrintString` (`KismetStringLibrary.Conv_DoubleToString` (`self.Health`)) true true (struct :`R` 0.75 :`G` 0.050861 :`B` 0.019531 :`A` 1.0))
    (if (`self.isDead`)
      (`PrimitiveComponent.SetCollisionResponseToChannel` _capsulecomponent "ECC_WorldDynamic" "ECR_Ignore")
      (`PrimitiveComponent.SetCollisionResponseToChannel` _capsulecomponent "ECC_Pawn" "ECR_Ignore")
      (`self.DetachFromControllerPendingDestroy`)
      (`SkeletalMeshComponent.PlayAnimation` (`self.Mesh`) "/Game/MyAssets/Blueprints/Characters/AnimationsFrog/frog_mutant_dying.frog_mutant_dying" false)
      ;[1 1 1] Spawn loot pickup at death location
      (`KismetSystemLibrary.Delay` 2.0)
      (`|SpawnActorFromClass` "/Game/MyAssets/Blueprints/ItemBPs/BP_FrogSkin.BP_FrogSkin_C" (`KismetMathLibrary.MakeTransform` (`SceneComponent.GetSocketLocation` (`self.Mesh`) "RightFoot")) "Undefined" "OverrideRootScale" null null)
      (`self.K2_DestroyActor`))))

(event `self.ReceiveBeginPlay`)

(fn `CalculateHealth`
  (params (delta :type "Float (double-precision)"))
  (bind _output_get (set `self.Health` (- (`self.Health`) delta)))
  (if (<= _output_get 0.0)
    (set `self.isDead` true)
    (`/Game/MyAssets/Blueprints/BP_HeroCharacter.UpdateKills` (cast `/Game/MyAssets/Blueprints/BP_HeroCharacter` (`GameplayStatics.GetPlayerCharacter` 0) :!pure true))))

(fn `TakeDamage`
  (`GameplayStatics.SpawnEmitterAtLocation` "/Game/StarterContent/Particles/P_Explosion.P_Explosion" (`self.K2_GetActorLocation`)))

(fn `UserConstructionScript`
  (bind _returnvalue (`PrimitiveComponent.CreateDynamicMaterialInstance` (`self.Mesh`) 0 null "None"))
  (bind _output_get (set `self.DynaMat` _returnvalue))
  (`MaterialInstanceDynamic.SetVectorParameterValue` _output_get "BodyColor" (`self.EnemyColor`)))