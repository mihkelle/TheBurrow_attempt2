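; BP_Door is a door actor that the player removes by interacting with it repeatedly.
; Overlap events on the Door_Collison component enable the actor's input while the player character is inside and disable it on exit.
; Each Interact press decrements the Attempts counter, and a press made when the counter is already zero destroys the door.
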(event `self.Door_Collison.OnComponentBeginOverlap`
  (params (OverlappedComponent :type "PrimitiveComponent Object Reference") (OtherActor :type "Actor Object Reference") (OtherComp :type "PrimitiveComponent Object Reference") (OtherBodyIndex :type Integer) (bFromSweep :type Boolean) (SweepResult :type "HitResult Structure (by ref)"))
  ;[1 1 1] En-/disable Inputs
  (if (== OtherActor (`GameplayStatics.GetPlayerCharacter` 0))
    (`self.EnableInput` (`GameplayStatics.GetPlayerController` 0))))

(event `self.Door_Collison.OnComponentEndOverlap`
  (params (OverlappedComponent :type "PrimitiveComponent Object Reference") (OtherActor :type "Actor Object Reference") (OtherComp :type "PrimitiveComponent Object Reference") (OtherBodyIndex :type Integer))
  ;[1 1 1] En-/disable Inputs
  (if (== OtherActor (`GameplayStatics.GetPlayerCharacter` 0))
    (`self.DisableInput` (`GameplayStatics.GetPlayerController` 0))))

(event `InputAction|Interact`
  (params (Key :type "Key Structure"))
  ;[1 1 1] Destroying the Door
  (:`Pressed`
    (if (== (`self.Attempts`) 0)
      (`self.K2_DestroyActor`)
      (else
        (bind _result (`/Engine/EditorBlueprintResources/StandardMacros.DecrementInt` (`self.Attempts`))
          (:`  `
            (set `self.Attempts` _result)))))))

(fn `UserConstructionScript`)