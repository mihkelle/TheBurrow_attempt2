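; BP_PickUp is a collectible item the player picks up with the Interact input while near it.
; Its TriggerBox enables input on the actor when the player character overlaps and disables it when they leave.
; On Interact, after a validity check, it destroys itself, increments the Collection counter on the Player character and plays a 2D sound.
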(event `self.TriggerBox.OnComponentBeginOverlap`
  (params (OverlappedComponent :type "PrimitiveComponent Object Reference") (OtherActor :type "Actor Object Reference") (OtherComp :type "PrimitiveComponent Object Reference") (OtherBodyIndex :type Integer) (bFromSweep :type Boolean) (SweepResult :type "HitResult Structure (by ref)"))
  ;[1 1 1] En-/Disable Inputs
  (if (== OtherActor (`GameplayStatics.GetPlayerCharacter` 0))
    (`self.EnableInput` (`GameplayStatics.GetPlayerController` 0))))

(event `self.TriggerBox.OnComponentEndOverlap`
  (params (OverlappedComponent :type "PrimitiveComponent Object Reference") (OtherActor :type "Actor Object Reference") (OtherComp :type "PrimitiveComponent Object Reference") (OtherBodyIndex :type Integer))
  ;[1 1 1] En-/Disable Inputs
  (if (== OtherActor (`GameplayStatics.GetPlayerCharacter` 0))
    (`self.DisableInput` (`GameplayStatics.GetPlayerController` 0))))

(event `InputAction|Interact`
  (params (Key :type "Key Structure"))
  ;[1 1 1] Collecting and item, Increasing nr of items collected
  (:`Pressed`
    (`/Engine/EditorBlueprintResources/StandardMacros.IsValid` (`self.Object`)
      (:`Is Valid`
        (`self.K2_DestroyActor`)
        (bind _asplayer (cast `/Game/StarterContent/WaterTests/Player` (`GameplayStatics.GetPlayerCharacter` 0)))
        (`/Engine/EditorBlueprintResources/StandardMacros.IncrementInt` (`/Game/StarterContent/WaterTests/Player.Collection` _asplayer)
          (:`  `
            (`GameplayStatics.PlaySound2D` null 1.0 1.0 0.0 null null)))))))

(fn `UserConstructionScript`)